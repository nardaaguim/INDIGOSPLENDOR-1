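; BORDER3 is a track segment for a runner game, randomly populated with a blocker, gold or silver.
; The construction script places a blocker at a left, front or right spawn point, or scatters several gold or silver child actors within the PickupArea box.
; When RUNNERAJNA overlaps EndTrigger, it calls AddMasterBorder on RUNNERGAMEMODE, then destroys itself after a short delay.
; GetAttachTransform exposes the AttachPoint's world transform.
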(event `self.ReceiveBeginPlay`
  (`self.SetSpawnPoint`))

(event `self.EndTrigger.OnComponentBeginOverlap`
  (params (OverlappedComponent :type "PrimitiveComponent Object Reference") (OtherActor :type "Actor Object Reference") (OtherComp :type "PrimitiveComponent Object Reference") (OtherBodyIndex :type Integer) (bFromSweep :type Boolean) (SweepResult :type "HitResult Structure (by ref)"))
  (cast `/Game/BLUEPRINTS/CHARACTERBP/RUNNERAJNA` OtherActor)
  (bind _asrunnergamemode (cast `/Game/GAMEMODE/RUNNERGAMEMODE` (`GameplayStatics.GetGameMode`)))
  (`/Game/GAMEMODE/RUNNERGAMEMODE.AddMasterBorder` _asrunnergamemode)
  (`KismetSystemLibrary.Delay` 1.0)
  (`self.K2_DestroyActor`))

(fn `GetAttachTransform`
  (returns (MasterBTrigger :type "Transform Structure"))
  (return (`SceneComponent.K2_GetComponentToWorld` (`self.AttachPoint`))))

(fn `SetSpawnPoint`
  (set `self.SpawnPoints` (`|MakeArray` (`SceneComponent.GetRelativeTransform` (`self.SpawnPointL`)) (`SceneComponent.GetRelativeTransform` (`self.SpawnPointF`)) (`SceneComponent.GetRelativeTransform` (`self.SpawnPointR`)))))

(fn `SpawnBlocker`
  (bind _spawnpoints (`self.SpawnPoints`))
  (`AddComponent|NODE_AddChildActorComponent-0` :`RelativeTransform` (`|GetArrayItem` _spawnpoints (`KismetMathLibrary.RandomIntegerInRange` 0 (`KismetArrayLibrary.Array_LastIndex` _spawnpoints)))))

(fn `SpawnGold`
  (bind _pickuparea (`self.PickupArea`))
  (for _ (range 3)
    (`AddComponent|NODE_AddChildActorComponent-1` :`RelativeTransform` (`KismetMathLibrary.Conv_VectorToTransform` (`KismetMathLibrary.RandomPointInBoundingBox` (`SceneComponent.RelativeLocation` _pickuparea) (`BoxComponent.BoxExtent` _pickuparea))))))

(fn `SpawnSilver`
  (bind _pickuparea (`self.PickupArea`))
  (for _ (range 7)
    (`AddComponent|NODE_AddChildActorComponent-2` :`RelativeTransform` (`KismetMathLibrary.Conv_VectorToTransform` (`KismetMathLibrary.RandomPointInBoundingBox` (`SceneComponent.RelativeLocation` _pickuparea) (`BoxComponent.BoxExtent` _pickuparea))))))

(fn `UserConstructionScript`
  (`self.SetSpawnPoint`)
  (switch `int` (`KismetMathLibrary.RandomIntegerInRange` 0 2)
    (:`0`
      (`self.SpawnBlocker`))
    (:`1`
      (`self.SpawnGold`))
    (:`2`
      (`self.SpawnSilver`))))